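; BP_LobbyGameMode is the lobby game mode that launches a match on the selected map.
; On BeginPlay it hides the first player controller's cursor and sets Game and UI input mode.
; StartGame uses the selected map index from BP_LobbyGameState to look up AvailableMaps.
; It then builds a ServerTravel console command with the listen option from that map's level asset, prints it and executes it.
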(event `self.ReceiveBeginPlay`
  (bind _returnvalue (`GameplayStatics.GetPlayerController` 0))
  (set `PlayerController.bShowMouseCursor` false _returnvalue)
  (`WidgetBlueprintLibrary.SetInputMode_GameAndUIEx` _returnvalue null))

(fn `Start Game`
  (`KismetSystemLibrary.PrintString` "Start Game Called!!")
  (bind _asbp_lobby_game_state (cast `/Game/Blueprint/BP_LobbyGameState` (`GameplayStatics.GetGameState`)))
  (bind _returnvalue (`KismetStringLibrary.Concat_StrStr` "ServerTravel " (`KismetSystemLibrary.Conv_SoftObjectReferenceToString` (`.MapLevelAsset` (break `MapSelectionData` (`|GetArrayItem` (`self.AvailableMaps`) (`LobbyGameState.SelectedMapIndex` _asbp_lobby_game_state))))) "?listen"))
  (`KismetSystemLibrary.PrintString` _returnvalue)
  (`KismetSystemLibrary.ExecuteConsoleCommand` _returnvalue null))

(fn `UserConstructionScript`)